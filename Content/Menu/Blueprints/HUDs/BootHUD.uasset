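; BootHUD is the boot-screen HUD that shows the game's splash and then starts authentication.
; On BeginPlay it creates the splash widget, plays its Splash animation and binds to that animation's finish event.
; When the animation ends, it swaps the splash for a load widget and calls Authenticate on the AuthenticationSubsystem with a hardcoded string.
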(event Custom|SplashAnimationEnded
  (Widget|RemovefromParent (stale EventBeginPlay _returnvalue))
  (bind _returnvalue (UserInterface|CreateWidget "/Game/Menu/Blueprints/Widgets/LoadWidget.LoadWidget_C" (Game|GetPlayerController 0)))
  (UserInterface|Viewport|AddtoViewport _returnvalue 0)
  (Class|AuthenticationSubsystem|Authenticate (Subsystems|GetAuthenticationSubsystem) "lixo"))

(event EventBeginPlay
  (bind _returnvalue (UserInterface|CreateWidget "/Game/Menu/Blueprints/Widgets/SplashWidget.SplashWidget_C" (Game|GetPlayerController 0)))
  (UserInterface|Viewport|AddtoViewport _returnvalue 0)
  (Class|UserWidget|BindtoAnimationFinished _returnvalue (Variables|/Game/Menu/Blueprints/Widgets/SplashWidget.SplashWidget_C|GetSplash _returnvalue) (delegate Custom|SplashAnimationEnded))
  (UserInterface|Animation|PlayAnimation _returnvalue (Variables|/Game/Menu/Blueprints/Widgets/SplashWidget.SplashWidget_C|GetSplash _returnvalue) 0.0 1 "Forward" 1.0 false))

(fn ConstructionScript)