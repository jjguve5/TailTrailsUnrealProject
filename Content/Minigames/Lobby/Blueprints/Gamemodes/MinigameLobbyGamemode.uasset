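; Game mode for the minigame lobby that tracks connected players and publishes lobby state through MinigameLobbyGamestate.
; On BeginPlay it copies the currently joining minigame's name from the MinigameHandlerSubsystem into the game state.
; Player logins and logouts update an AllPlayers list, then tell the game state to refresh its player list.
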(event Custom|Update_PlayerList
  (bind _asminigame_lobby_gamestate (Utilities|Casting|CastToMinigameLobbyGamestate (Game|GetGameState)))
  (Default|UpdatePlayerList _asminigame_lobby_gamestate))

(event EventBeginPlay
  (bind _asminigame_lobby_gamestate (Utilities|Casting|CastToMinigameLobbyGamestate (Game|GetGameState)))
  (Variables|/Game/Minigames/Lobby/Blueprints/Gamestates/MinigameLobbyGamestate.MinigameLobbyGamestate_C|SetMinigameName _asminigame_lobby_gamestate (Class|MinigameHandlerSubsystem|GetCurrentJoiningMinigameName (Subsystems|GetMinigameHandlerSubsystem))))

(event EventPostLogin
  (params (NewPlayer :type Player%20Controller%20Object%20Reference))
  (Utilities|Array|Add (Variables|Default|GetAllPlayers) NewPlayer)
  (CallFunction|UpdatePlayerList))

(event EventOnLogout
  (params (ExitingController :type Controller%20Object%20Reference))
  (bind _asplayer_controller (Utilities|Casting|CastToPlayerController ExitingController))
  (Utilities|Array|RemoveItem (Variables|Default|GetAllPlayers) _asplayer_controller)
  (CallFunction|UpdatePlayerList))

(fn ConstructionScript)